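; BP_HealthComponent is a component that tracks health and death for its owning actor.
; On BeginPlay it binds to the owner's OnTakeAnyDamage event and subtracts incoming damage from its current health.
; When health reaches zero or below, it sets IsDead and fires the OnDeath dispatcher, and the flag makes it ignore any further damage.
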(event `self.ReceiveBeginPlay`
  (add `Actor.OnTakeAnyDamage` (`self.GetOwner`) (delegate `OnTakeAnyDamage`)))

(event `OnTakeAnyDamage`
  (params (DamagedActor :type "Actor Object Reference") (Damage :type "Float (double-precision)") (DamageType :type "DamageType Object Reference") (InstigatedBy :type "Controller Object Reference") (DamageCauser :type "Actor Object Reference"))
  (if (not (`self.isDead`))
    (bind _output_get (set `self.CurrentHealths` (- (`self.CurrentHealths`) Damage)))
    (if (<= _output_get 0.0)
      (set `self.isDead` true)
      (`self.OnDeath`))))