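; Long sword weapon Blueprint that overrides Attack to hit enemies in an arc in front of its owner.
; It fans line traces on the Visibility channel at one-degree steps across AttackRotation, reaching BladeRadius, with debug drawing on.
; Each step adds unique BP_EnemyCharacter hits to HitedEnemies, calls DamageEnemies, plays the attack montage and sets a timer to the montage's length.
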(fn `Attack`
  (locals (_StartRot :type "Float (double-precision)" :default 0.0))
  (bind _returnvalue (`self.K2_GetActorLocation` (`self.GetOwner`)))
  (`parent.Attack`)
  (set `local._StartRot` (- (.yaw (`self.K2_GetActorRotation` (`self.GetOwner`))) (/ (`self.AttackRotation`) 2.0)))
  (for _index (range 1 (+ (`KismetMathLibrary.FTrunc` (`self.AttackRotation`)) 1))
    (bind _outhits (`KismetSystemLibrary.LineTraceMulti` :`Start` _returnvalue :`End` (+ (* (`KismetMathLibrary.GetForwardVector` (`KismetMathLibrary.MakeRotator` 0.0 0.0 (+ (`KismetMathLibrary.Conv_IntToDouble` _index) (`local._StartRot`)))) (`self.BladeRadius`)) _returnvalue) :`TraceChannel` "TraceTypeQuery1" :`DrawDebugType` "ForDuration"))
    (for _array_element _outhits
      (bind _asbp_enemy_character (cast `/Game/Blueprints/BP_EnemyCharacter` (`.HitActor` (`GameplayStatics.BreakHitResult` _array_element))))
      (`KismetArrayLibrary.Array_AddUnique` (`self.HitedEnemies`) _asbp_enemy_character))
    (`self.DamageEnemies`)
    (bind _returnvalue_2 (`Character.PlayAnimMontage` (cast `Character` (`self.GetOwner`) :!pure true) "/Game/Meshes/StaticMeshes/Weapons/LongSword/Animations/AnimMontages/AnimMontage_BaseAttack_LongSword.AnimMontage_BaseAttack_LongSword" 1.0 "None"))
    (`KismetSystemLibrary.K2_SetTimerDelegate` (`|CreateDelegate` :!event `EndAttack`) _returnvalue_2)))

(fn `UserConstructionScript`
  (`parent.UserConstructionScript`))