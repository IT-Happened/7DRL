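; Base weapon that runs melee-style combo attacks for its owning character, with getters for damage, range and attack state.
; Each combo step starts its configured attack objects after proportional delays and plays a random montage rate-scaled to the step's duration.
; Timers mark the step's end and a late combo point, while saved-attack flags let buffered input chain the next step.
; Player-controlled owners cannot move until EndAttack resets the combo.
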(event `self.ReceiveBeginPlay`
  (for _array_element (`self.ComboAttacks`)
    (for _array_element_2 (`.Attacks` (break `ComboAttack` _array_element))
      (`BaseAttackType.Initialize` (`.Attacks` (break `Attack` _array_element_2)) self))))

(fn `Attack`
  (bind _ascharacter (cast `Character` (`self.GetOwner`) :!pure true))
  (bind _canattack (message `/Game/Blueprints/Weapons/BI_Attack.CanAttack` (`self.GetOwner`)))
  (if _canattack
    (set `self.isAttacking` true)
    (bind _result (`/Engine/EditorBlueprintResources/StandardMacros.IncrementInt` (`self.AttackCount`))
      (:`  `
        (cast `/Game/Blueprints/Player/BP_PlayerController` (`Pawn.GetController` _ascharacter)
          (:`then`
            (`CharacterMovementComponent.DisableMovement` (`Character.CharacterMovement` _ascharacter)))
          (:`CastFailed`
            _))
        (bind (_attacks _attacktimemultiple _attackanimations) (break `ComboAttack` (`|GetArrayItem` (`self.ComboAttacks`) _result)))
        (set `self.AttackTime` (* _attacktimemultiple (`self.BaseAttackTime`)))
        (for _array_element _attacks
          (`self.UseAttack` _array_element))
        (bind _output (`|GetArrayItem` _attackanimations (`KismetMathLibrary.RandomInteger` (`KismetArrayLibrary.Array_Length` _attackanimations))))
        (`Character.PlayAnimMontage` (cast `Character` (`self.GetOwner`) :!pure true) _output (`self.Calculate Montage Play Rate` _output (`self.AttackTime`)) "None")
        (bind _returnvalue (`KismetSystemLibrary.K2_SetTimerDelegate` (`|CreateDelegate` :!event `EndAttack`) (`self.AttackTime`)))
        (set `self.EndAttackTimer` _returnvalue)
        (if (< (+ (`self.AttackCount`) 1) (`KismetArrayLibrary.Array_Length` (`self.ComboAttacks`)))
          (`KismetSystemLibrary.K2_SetTimerDelegate` (`|CreateDelegate` :!event `ContinueCombo`) (* (`self.AttackTime`) 0.7)))))))

(fn `Calculate Montage Play Rate`
  (params (Target :type "AnimSequenceBase Object Reference") (TimeToPlay :type "Float (double-precision)"))
  (returns (Rate :type "Float (double-precision)"))
  (bind _returnvalue (`AnimSequenceBase.GetPlayLength` Target))
  (return (/ _returnvalue TimeToPlay)))

(fn `ContinueCombo`
  (if (`self.IsSavingAttack`)
    (`self.Attack`)
    (set `self.IsSavingAttack` false)))

(fn `EndAttack`
  (bind _ascharacter (cast `Character` (`self.GetOwner`) :!pure true))
  (if (`self.isAttacking`)
    (set `self.isAttacking` false)
    (set `self.AttackCount` -1)
    (`Character.StopAnimMontage` (cast `Character` (`self.GetOwner`) :!pure true) null)
    (cast `/Game/Blueprints/Player/BP_PlayerController` (`Pawn.GetController` _ascharacter)
      (:`then`
        (`CharacterMovementComponent.SetMovementMode` (`Character.CharacterMovement` _ascharacter) "MOVE_Walking" 0))
      (:`CastFailed`
        _))
    (`self.AttackEnd`)))

(fn `GetAttackTime`
  (returns (AttackTime :type "Float (double-precision)"))
  (return (`self.AttackTime`)))

(fn `GetTagsToIgnore`
  (returns (ReturnValue :type "Array of Name"))
  (return))

(fn `GetWeaponDamage`
  (returns (ReturnValue :type "Map of BaseDamageType Class Reference to Float (double-precision)"))
  (return (`self.Damages`)))

(fn `GetWeaponDistance`
  (returns (ReturnValue :type "Float (double-precision)"))
  (return (`self.AttackDistance`)))

(fn `IsDrawDebug`
  (returns (ReturnValue :type Boolean))
  (return false))

(fn `IsWeaponAttacking`
  (returns (isAttacking :type Boolean))
  (return (`self.isAttacking`)))

(fn `SaveAttack`
  (params (IsSavingAttack :type Boolean))
  (if IsSavingAttack
    (if (not (`self.IsSavingAttack`))
      (if (== (+ (`self.AttackCount`) 1) (`KismetArrayLibrary.Array_LastIndex` (`self.ComboAttacks`)))
        (set `self.LastAttackSave` true)
        (else
          (set `self.IsSavingAttack` true))))
    (else
      (set `self.IsSavingAttack` false)
      (set `self.LastAttackSave` false))))

(fn `SaveLastAttack`
  (if (and (== (+ (`self.AttackCount`) 1) (`KismetArrayLibrary.Array_LastIndex` (`self.ComboAttacks`))) (`self.LastAttackSave`))
    (set `self.IsSavingAttack` true)))

(fn `UseAttack`
  (params (Attack :type "Attack Structure"))
  (bind (_delaytime _attacks) (break `Attack` Attack))
  (`/Engine/EditorBlueprintResources/StandardMacros.IsValid` _attacks
    (:`Is Valid`
      (`BaseAttackType.StartUseAttack` _attacks (* _delaytime (`self.AttackTime`))))))

(fn `UserConstructionScript`)