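; Player pistol weapon that extends its parent weapon with a limited ammo pool and a charge-based refill.
; Attacks are blocked at zero ammo, and projectile attack actions start a one-shot timer scaled to the attack's pre-attack delay.
; AddAmmoСharge builds fractional charge while below max ammo, converting a full charge into one round.
; Spending or gaining a round updates the owning BP_PlayerCharacter's HUD.
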(fn `AddAmmo`
  (`/Engine/EditorBlueprintResources/StandardMacros.IncrementInt` (`self.Ammo`)
    (:`  `
      (bind _asbp_player_character (cast `/Game/Blueprints/Player/BP_PlayerCharacter` (`self.GetOwner`)))
      (`/Game/UI/WBP_PlayerHUD.SetAmmo` (`/Game/Blueprints/Player/BP_PlayerCharacter.PlayerHUD` _asbp_player_character) (`self.Ammo`) (`self.MaxAmmo`)))))

(fn `AddAmmoСharge`
  (if (!= (`self.Ammo`) (`self.MaxAmmo`))
    (bind _output_get (set `self.AmmoCharge` (+ (`self.AmmoCharge`) 0.2)))
    (if (`KismetMathLibrary.NearlyEqual_FloatFloat` _output_get 1.0 0.001)
      (`self.AddAmmo`)
      (set `self.AmmoCharge` 0.0))))

(fn `IsDrawDebug`
  (returns (ReturnValue :type Boolean))
  (return false))

(fn `Try Attack`
  (params (Action :type "EAttackActions Enum" :default "AA_NONE"))
  (if (> (`self.Ammo`) 0)
    (`parent.Try Attack` Action)))

(fn `Use Attack Action`
  (params (AttackAction :type "Attack Structure"))
  (bind (_delaytime _attacks) (break `Attack` AttackAction))
  (`parent.Use Attack Action` AttackAction)
  (`/Engine/EditorBlueprintResources/StandardMacros.IsValid` _attacks
    (:`Is Valid`
      (cast `ProjectileAttack` _attacks)
      (`KismetSystemLibrary.K2_SetTimerDelegate` (`|CreateDelegate` :!event `UseAmmo`) (* _delaytime (`self.GetAttackTime`))))))

(fn `UseAmmo`
  (`/Engine/EditorBlueprintResources/StandardMacros.DecrementInt` (`self.Ammo`)
    (:`  `
      (bind _asbp_player_character (cast `/Game/Blueprints/Player/BP_PlayerCharacter` (`self.GetOwner`)))
      (`/Game/UI/WBP_PlayerHUD.SetAmmo` (`/Game/Blueprints/Player/BP_PlayerCharacter.PlayerHUD` _asbp_player_character) (`self.Ammo`) (`self.MaxAmmo`)))))

(fn `UserConstructionScript`
  (`parent.UserConstructionScript`))