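; Ranged weapon Blueprint that fires a projectile when its owner attacks.
; Attack calls the parent logic, then Shoot, which plays the pistol fire montage on the owning Character and spawns BP_Projectile just below the weapon, facing the owner's rotation.
; The projectile receives the owner and the weapon's Damage.
; EndAttack runs immediately without waiting for the montage, and is called in both Shoot and Attack.
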(fn `Attack`
  (`parent.Attack`)
  (`self.Shoot`)
  (`self.EndAttack`))

(fn `Shoot`
  (`Character.PlayAnimMontage` (cast `Character` (`self.GetOwner`) :!pure true) "/Game/Meshes/StaticMeshes/Weapons/Pistol/Animations/AnimMontages/AnimMontage_Fire_Pistol.AnimMontage_Fire_Pistol" 1.0 "None")
  (`|SpawnActorFromClass` "/Game/Blueprints/Weapons/BP_Projectile.BP_Projectile_C" (`KismetMathLibrary.MakeTransform` (- (`self.K2_GetActorLocation`) (0.0 0.0 50.0)) (`self.K2_GetActorRotation` (`self.GetOwner`))) "AlwaysSpawn" "OverrideRootScale" (`self.GetOwner`) (`self.Damage`) null)
  (`self.EndAttack`))

(fn `UserConstructionScript`
  (`parent.UserConstructionScript`))