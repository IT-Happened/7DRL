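; Level exit trigger that moves the player on to the next dungeon run or back to the menu.
; When the player pawn overlaps its Box, it increments LevelCount on the globals game instance, so progress persists across level loads.
; It reopens TestDungeonGenerator while the count is under the level limit, otherwise it opens BP_menu.
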(event `self.Box.OnComponentBeginOverlap`
  (params (OverlappedComponent :type "PrimitiveComponent Object Reference") (OtherActor :type "Actor Object Reference") (OtherComp :type "PrimitiveComponent Object Reference") (OtherBodyIndex :type Integer) (bFromSweep :type Boolean) (SweepResult :type "HitResult Structure (by ref)"))
  (if (== OtherActor (`GameplayStatics.GetPlayerPawn` 0))
    (bind _asglobals (cast `/Game/Blueprints/Level/globals` (`GameplayStatics.GetGameInstance`)))
    (bind _result (`/Engine/EditorBlueprintResources/StandardMacros.IncrementInt` (`/Game/Blueprints/Level/globals.level_count` _asglobals))
      (:`  `
        (if (< _result 10)
          (`GameplayStatics.OpenLevel` "TestDungeonGenerator")
          (else
            (`GameplayStatics.OpenLevel` "BP_menu")))))))

(fn `UserConstructionScript`)