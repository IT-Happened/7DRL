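; BP_LevelEnd is a level exit trigger that advances the run or ends the game when the player pawn overlaps its Box.
; Each overlap increments LevelCount in BP_GameInstance, so progress persists across level loads.
; While the count is below a fixed limit it opens the TestDungeonGenerator level again; otherwise it clears all widgets and shows the WBP_Titles_Final screen.
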(event `self.Box.OnComponentBeginOverlap`
  (params (OverlappedComponent :type "PrimitiveComponent Object Reference") (OtherActor :type "Actor Object Reference") (OtherComp :type "PrimitiveComponent Object Reference") (OtherBodyIndex :type Integer) (bFromSweep :type Boolean) (SweepResult :type "HitResult Structure (by ref)"))
  (if (== OtherActor (`GameplayStatics.GetPlayerPawn` 0))
    (bind _asbp_game_instance (cast `/Game/Blueprints/Global/BP_GameInstance` (`GameplayStatics.GetGameInstance`)))
    (bind _result (`/Engine/EditorBlueprintResources/StandardMacros.IncrementInt` (`/Game/Blueprints/Global/BP_GameInstance.level_count` _asbp_game_instance))
      (:`  `
        (if (< _result 5)
          (`GameplayStatics.OpenLevel` "TestDungeonGenerator")
          (else
            (`WidgetLayoutLibrary.RemoveAllWidgets`)
            (bind _returnvalue (`|CreateWidget` "/Game/UI/Titles/WBP_Titles_Final.WBP_Titles_Final_C" (`GameplayStatics.GetPlayerController` 0)))
            (`UserWidget.AddToViewport` _returnvalue 0)))))))

(fn `UserConstructionScript`)