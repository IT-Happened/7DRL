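; BP_SceneGenerator is an early procedural room layout generator that spawns static mesh floors when play begins.
; It places a start room mesh, then generates a random handful of vectors within the room scale limits.
; MoveGeometryLocation accumulates these vectors into a chain of locations for template floors, without scaling them.
; Seeded split, filter and space-partition helpers are uncalled or unfinished, and the construction script has no effect.
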(event `self.ReceiveBeginPlay`
  (bind _returnvalue (`|SpawnActorFromClass` "/Script/Engine.StaticMeshActor" (`KismetMathLibrary.Conv_VectorToTransform` (`self.StartRoom`)) "Undefined" "OverrideRootScale" null null))
  (`StaticMeshComponent.SetStaticMesh` (`StaticMeshActor.StaticMeshComponent` _returnvalue) "/Game/Meshes/StaticMeshes/Rooms/SM_Room_1x1_A.SM_Room_1x1_A")
  (bind _roomsgeometryscale (`self.Generate Vector Array` (`self.MinimumRoomScale`) (`self.MaximumRoomScale`)))
  (bind _movedrooms (`self.MoveGeometryLocation` _roomsgeometryscale))
  (for _array_element _movedrooms
    (bind _returnvalue_2 (`|SpawnActorFromClass` "/Script/Engine.StaticMeshActor" (`KismetMathLibrary.Conv_VectorToTransform` _array_element) "Undefined" "OverrideRootScale" null null))
    (`StaticMeshComponent.SetStaticMesh` (`StaticMeshActor.StaticMeshComponent` _returnvalue_2) "/Game/Meshes/StaticMeshes/Enviroment/TemplateFloor.TemplateFloor"))
  (`KismetSystemLibrary.PrintText` (`|FormatText` "x = {1} y = {2} z = {3}" (.x _array_element) (.y _array_element) (.z _array_element)) true true (struct :`G` 0.66 :`B` 1.0 :`A` 1.0) 120.0))

(fn `FilterVectorArrayBySquare`
  (params (InputArray :type "Array of Vector Structure") (MinimalVector :type "Vector Structure"))
  (returns (FilteredArray :type "Array of Vector Structure"))
  (locals (ResultArray :type "Array of Vector Structure"))
  (for _array_element InputArray
    (if (and (> (.x _array_element) (.x MinimalVector)) (> (.y _array_element) (.y MinimalVector)))
      (`KismetArrayLibrary.Array_Append` (`local.ResultArray`) (`|MakeArray` _array_element))))
  (return (`local.ResultArray`)))

(fn `Generate Vector Array`
  (params (MinimumRoomVector :type "Vector Structure") (MaximumRoomVector :type "Vector Structure"))
  (returns (RoomsGeometryScale :type "Array of Vector Structure"))
  (locals (ResultGeometryScale :type "Array of Vector Structure"))
  (for _ (range (+ (`KismetMathLibrary.RandomIntegerInRange` 4 10) 1))
    (bind _newroomsize (`self.GenerateArrayOfVector` MinimumRoomVector MaximumRoomVector))
    (`KismetArrayLibrary.Array_Append` (`local.ResultGeometryScale`) (`|MakeArray` _newroomsize)))
  (return (`local.ResultGeometryScale`)))

(fn `GenerateArrayOfVector`
  (params (minimum :type "Vector Structure") (maximum :type "Vector Structure"))
  (returns (NewRoomSize :type "Vector Structure"))
  (return (`KismetMathLibrary.MakeVector` (`KismetMathLibrary.RandomFloatInRange` (.x minimum) (.x maximum)) (`KismetMathLibrary.RandomFloatInRange` (.y minimum) (.y maximum)) (.z minimum))))

(fn `GenerateSpacePartition`
  (params (Square :type "Vector Structure"))
  (locals (isVerticalDirection :type Boolean) (isXPosition :type Boolean) (ratio :type "Float (double-precision)"))
  (set `local.isVerticalDirection` (`KismetMathLibrary.RandomBool`))
  (set `local.isXPosition` (`KismetMathLibrary.RandomBool`))
  (set `local.ratio` (`KismetMathLibrary.RandomFloatInRange` 0.3 0.7))
  (if (`local.isXPosition`)
    _))

(fn `GetRandomStream`
  (returns (RandomFloatResult :type "RandomStream Structure"))
  (locals (stream :type "RandomStream Structure"))
  (bind _output_get (set `local.stream` (`KismetMathLibrary.MakeRandomStream` (`self.Seed`))))
  (return _output_get))

(fn `MoveGeometryLocation`
  (params (RoomsGeometry :type "Array of Vector Structure"))
  (returns (MovedRooms :type "Array of Vector Structure"))
  (locals (TemperaryRoom :type "Vector Structure") (MovedRoomArray :type "Array of Vector Structure") (`Total Square` :type "Vector Structure"))
  (`KismetArrayLibrary.Array_Append` (`local.MovedRoomArray`) (`|MakeArray` (`|GetArrayItem` RoomsGeometry)))
  (for _index (range 1 (`KismetArrayLibrary.Array_Length` RoomsGeometry))
    (bind _output (`|GetArrayItem` (`local.MovedRoomArray`) (- _index 1)))
    (`KismetArrayLibrary.Array_Append` (`local.MovedRoomArray`) (`|MakeArray` (`KismetMathLibrary.MakeVector` (.x (+ _output (`|GetArrayItem` RoomsGeometry _index))) (.y (+ _output (`|GetArrayItem` RoomsGeometry _index))) (.z _output)))))
  (return (`local.MovedRoomArray`)))

(fn `NewSeed`
  (returns (NewRandomSeed :type Integer))
  (bind _output_get (set `self.Seed` (`KismetMathLibrary.RandomInteger` 0)))
  (return _output_get))

(fn `SplitVector`
  (params (InputGeometry :type "Vector Structure (by ref)"))
  (returns (Array :type "Array of Vector Structure"))
  (bind _x (.x InputGeometry))
  (bind _y (.y InputGeometry))
  (bind _z (.z InputGeometry))
  (bind _randomfloatresult (`self.GetRandomStream`))
  (if (`KismetMathLibrary.RandomBool`)
    (bind _returnvalue (`KismetMathLibrary.RandomFloatInRangeFromStream` 0.0 1.0 _randomfloatresult))
    (bind _returnvalue_2 (* _returnvalue _x))
    (return (`|MakeArray` (`KismetMathLibrary.MakeVector` _returnvalue_2 _y _z) (`KismetMathLibrary.MakeVector` (- _x _returnvalue_2) _y _z)))
    (else
      (bind _returnvalue_3 (* _returnvalue _y))
      (return (`|MakeArray` (`KismetMathLibrary.MakeVector` _x _returnvalue_3 _z) (`KismetMathLibrary.MakeVector` _x (- _y _returnvalue_3) _z))))))

(fn `UserConstructionScript`
  (for _ (range 5)
    (bind _returnvalue (message `MovieSceneTransformOrigin.BP_GetTransformOrigin` (`self.DefaultSceneRoot`)))))