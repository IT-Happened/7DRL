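; Base enemy character that runs a behavior tree on possession and can be stunned, blocking attacks for a timed montage.
; Health component events feed an overhead widget's health bar, plus armor when the enemy has any.
; Death disables capsule collision, hides the widget, starts ragdoll physics and destroys the controller.
; If a player dealt the final damage, they receive pistol ammo, kill credit and armor, and the enemy is destroyed.
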(event `self.ReceivePossessed`
  (params (NewController :type "Controller Object Reference"))
  (`AIController.RunBehaviorTree` (cast `AIController` NewController :!pure true) (`self.BTAsset`)))

(event `self.ReceiveBeginPlay`
  (bind _bp_healthcomponent (`self.BP_HealthComponent`))
  (add `/Game/Blueprints/Components/BP_HealthComponent.HealthChanged` (`self.BP_HealthComponent`) (`|CreateDelegate` :!event `OnHealthChanged`))
  (`self.OnHealthChanged`)
  (`|ExecutionSequence`
    (:`then_0`
      (if (> (`.MaxArmor` (`/Game/Blueprints/Components/BP_HealthComponent.GetArmor` _bp_healthcomponent)) 0.0)
        (add `/Game/Blueprints/Components/BP_HealthComponent.ArmorChanged` _bp_healthcomponent (`|CreateDelegate` :!event `OnArmorChanged`))
        (`self.OnArmorChanged`)))
    (:`then_1`
      (add `/Game/Blueprints/Components/BP_HealthComponent.Death` (`self.BP_HealthComponent`) (`|CreateDelegate` :!event `OnDeath`)))))

(event `CharacterInterface.StunCharacter`
  (params (StunTime :type "Float (single-precision)"))
  (if (not (`self.IsStun`))
    (`/Game/Blueprints/Weapons/BP_BaseWeapon.EndAttack` (`/Game/Blueprints/Components/BP_WeaponComponent.GetCurrentWeapon` (`self.BP_WeaponComponent`)))
    (set `self.IsStun` true)
    (`|PlayMontage` (`self.Mesh`) (`self.StunMontage`)
      (:`then`
        (`KismetSystemLibrary.K2_SetTimerDelegate` (delegate `OnStunEnd`) StunTime)))))

(event `OnStunEnd`
  (if (`self.IsStun`)
    (set `self.IsStun` false)
    (`self.StopAnimMontage` (`self.StunMontage`))))

(fn `CanAttack`
  (returns (CanAttack :type Boolean))
  (return (not (`self.IsStun`))))

(fn `OnArmorChanged`
  (bind (_currentarmor _maxarmor) (`/Game/Blueprints/Components/BP_HealthComponent.GetArmor` (`self.BP_HealthComponent`)))
  (bind _aswbp_enemy_health (cast `/Game/UI/WBP_EnemyHealth` (`WidgetComponent.GetWidget` (`self.Widget`))))
  (`/Game/UI/WBP_EnemyHealth.SetArmor` _aswbp_enemy_health (/ _currentarmor _maxarmor)))

(fn `OnDeath`
  (params (IsGreatDeath :type Boolean))
  (`|ExecutionSequence`
    (:`then_0`
      (`PrimitiveComponent.SetCollisionEnabled` (`self.CapsuleComponent`) "NoCollision")
      (`SceneComponent.SetHiddenInGame` (`self.Widget`) true false)
      (`PrimitiveComponent.SetSimulatePhysics` (`self.Mesh`) true)
      (`self.K2_DestroyActor` (`self.GetController`)))
    (:`then_1`
      (bind _asplayer_controller (cast `PlayerController` (`/Game/Blueprints/Components/BP_HealthComponent.LastDamageInstigator` (`self.BP_HealthComponent`))))
      (bind _asbp_player_character (cast `/Game/Blueprints/Player/BP_PlayerCharacter` (`Controller.K2_GetPawn` _asplayer_controller)))
      (`/Game/Blueprints/Player/BP_PlayerCharacter.Add Ammo For Pistol` _asbp_player_character)
      (`/Game/Blueprints/Player/BP_PlayerCharacter.AddKilledEnemies` _asbp_player_character)
      (bind _bp_healthcomponent (`/Game/Blueprints/Player/BP_PlayerCharacter.BP_HealthComponent` _asbp_player_character))
      (`/Game/Blueprints/Components/BP_HealthComponent.SetArmor` _bp_healthcomponent (+ (`/Game/Blueprints/Components/BP_HealthComponent.GetArmor` _bp_healthcomponent) (`self.ArmorToRestore`)))
      (`self.K2_DestroyActor`))))

(fn `OnHealthChanged`
  (bind (_currenthealth _maxhealth) (`/Game/Blueprints/Components/BP_HealthComponent.GetHealth` (`self.BP_HealthComponent`)))
  (bind _aswbp_enemy_health (cast `/Game/UI/WBP_EnemyHealth` (`WidgetComponent.GetWidget` (`self.Widget`))))
  (`/Game/UI/WBP_EnemyHealth.SetHealths` _aswbp_enemy_health (/ _currenthealth _maxhealth)))

(fn `UserConstructionScript`)